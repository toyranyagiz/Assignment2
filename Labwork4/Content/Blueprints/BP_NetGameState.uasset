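; BP_NetGameState is a game state Blueprint that handles the end of a team-based networked match and the result display.
; On victory, it compares each player state's TeamID with the winning player's and calls the won or lost handler on that player's BP_NetAvatar.
; It then shows a W_GameResults widget naming the winning team, stored in MessageWidget so that restart can remove it.
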(event `self.OnVictory`
  (bind _returnvalue (`self.GetPlayerStateByIndex` (`self.WinningPlayer`)))
  (for _array_element (`self.PlayerArray`)
    (bind _asnet_player_state (cast `NetPlayerState` _array_element))
    (bind (_data_nickname _data_customizationdata _data_teamid) (break `SPlayerInfo` (`NetPlayerState.Data` _asnet_player_state)))
    (if (`|EnumEquality` _data_teamid (`.TeamID` (break `SPlayerInfo` (`NetPlayerState.Data` _returnvalue))))
      (bind _asbp_net_avatar (cast `/Game/Blueprints/BP_NetAvatar` (`PlayerState.PawnPrivate` _asnet_player_state) :!pure true))
      (`/Game/Blueprints/BP_NetAvatar.OnPlayerWon` _asbp_net_avatar)
      (else
        (`/Game/Blueprints/BP_NetAvatar.OnPlayerLost` _asbp_net_avatar))))
  (`self.ShowResultMessage`))

(event `self.OnRestart`
  (`Widget.RemoveFromParent` (`self.MessageWidget`)))

(fn `ShowResultMessage`
  (bind _returnvalue (`self.GetPlayerStateByIndex` (`self.WinningPlayer`)))
  (bind _returnvalue_2 (`|CreateWidget` "/Game/Blueprints/UMG/W_GameResults.W_GameResults_C" null (`|FormatText` "{team} WINS!" (`|GetEnumeratorNameAsString` (`.TeamID` (break `SPlayerInfo` (`NetPlayerState.Data` _returnvalue)))))))
  (bind _output_get (set `self.MessageWidget` _returnvalue_2))
  (`UserWidget.AddToViewport` _returnvalue_2 0)
  (`UserWidget.AddToViewport` _output_get 0))

(fn `UserConstructionScript`)